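; BP_IteminGame is an in-world item pickup display that shows an item's icon and name.
; On BeginPlay it fills a Paper2D sprite and a text render from the CurrentItem data.
; Each Tick it rotates the text toward the top-down controller's camera, billboarding the name label so it stays readable.
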(event EventBeginPlay
  (Rendering|Components|Sprite|SetSprite (Variables|Default|GetPaperSprite) (Variables|/Game/Blueprint/Data/BP_DA_Item.BP_DA_Item_C|GetIcone (Variables|Default|GetCurrentItem)))
  (Rendering|Components|TextRender|SetText (Variables|Default|GetTextRender) (Variables|/Game/Blueprint/Data/BP_DA_Item.BP_DA_Item_C|GetName (Variables|Default|GetCurrentItem))))

(event EventTick
  (params (DeltaSeconds :type Float%20%28single-precision%29))
  (Transformation|SetWorldRotation (Variables|Default|GetTextRender) (Math|Rotator|FindLookatRotation (Transformation|GetWorldLocation (Variables|Default|GetTextRender)) (Camera|GetCameraLocation (Variables|/Script/Engine.PlayerController|GetPlayerCameraManager (CallFunction|GetTopDownController)))) false false))

(fn ConstructionScript)