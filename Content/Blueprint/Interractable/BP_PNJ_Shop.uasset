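; BP_PNJ_Shop is an interactable shop NPC that opens a shop screen when the player interacts with it.
; Interraction blends the camera to the NPC, shows its widget component, initializes WBP_Shop with a self reference and disables movement on the top-down controller.
; ExitShop hides the widget, re-enables movement and blends the camera back to the controlled pawn.
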(event Custom|ExitShop
  (bind _player_controller (CallFunction|GetTopDownController))
  (Rendering|SetVisibility (Variables|Default|GetWidget) false false)
  (Variables|/Game/Blueprint/BP_TopDownController.BP_TopDownController_C|SetShouldMove (CallFunction|GetTopDownController) true)
  (Game|Player|SetViewTargetwithBlend _player_controller (Pawn|GetControlledPawn _player_controller) 1.0 "VTBlend_Linear" 1.0 false))

(event EventInterraction
  (bind _widget (Variables|Default|GetWidget))
  (Game|Player|SetViewTargetwithBlend (CallFunction|GetTopDownController) self 1.0 "VTBlend_Linear" 1.0 false)
  (Rendering|SetVisibility _widget true false)
  (bind _aswbp_shop (Utilities|Casting|CastToWBP_Shop (UserInterface|GetWidget _widget)))
  (Default|InitializeShop _aswbp_shop self)
  (Variables|/Game/Blueprint/BP_TopDownController.BP_TopDownController_C|SetShouldMove (CallFunction|GetTopDownController) false))

(fn ConstructionScript
  (|CallParentFunction))