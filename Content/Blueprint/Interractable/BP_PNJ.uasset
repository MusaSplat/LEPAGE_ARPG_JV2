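; BP_PNJ is an interactable NPC that shows a text line and takes over the camera when the player interacts with it.
; Its Interraction event uses a FlipFlop to alternate between entering and leaving the interaction.
; Entering reveals the TextRender, blends the view target to the NPC and disables movement through the top-down controller's ShouldMove flag.
; Leaving hides the text, blends back to the controlled pawn and restores movement.
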(event EventBeginPlay)

(event Collision|EventActorBeginOverlap
  (params (OtherActor :type Actor%20Object%20Reference)))

(event EventTick
  (params (DeltaSeconds :type Float%20%28single-precision%29)))

(event EventInterraction
  (bind _player_controller (CallFunction|GetTopDownController))
  (bind _player_controller_2 (CallFunction|GetTopDownController))
  (Utilities|FlowControl|FlipFlop
    (:A
      (Rendering|SetVisibility (Variables|Default|GetTextRender1) true false)
      (Game|Player|SetViewTargetwithBlend _player_controller self 1.0 "VTBlend_Linear" 0.0 false)
      (Variables|/Game/Blueprint/BP_TopDownController.BP_TopDownController_C|SetShouldMove _player_controller false))
    (:B
      (Rendering|SetVisibility (Variables|Default|GetTextRender1) false false)
      (Game|Player|SetViewTargetwithBlend _player_controller_2 (Pawn|GetControlledPawn _player_controller_2) 1.0 "VTBlend_Linear" 0.0 false)
      (Variables|/Game/Blueprint/BP_TopDownController.BP_TopDownController_C|SetShouldMove _player_controller_2 true))))

(fn ConstructionScript)

(fn NewFunction)