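; BP_PNJ is an NPC that toggles a dialogue-style view when interacted with.
; Its Interract event uses a FlipFlop to show TextRender1 and blend the top-down controller's view target to the NPC, then on the next call hide the text and blend back to the controlled pawn.
; The construction script and NewFunction are empty.
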(event Custom|Event%20Interract
  (bind _player_controller (CallFunction|GetTopDownController))
  (Utilities|FlowControl|FlipFlop
    (:A
      (Rendering|SetVisibility (Variables|Default|GetTextRender1) true false)
      (Game|Player|SetViewTargetwithBlend (CallFunction|GetTopDownController) self 0.5 "VTBlend_Linear" 0.0 false))
    (:B
      (Rendering|SetVisibility (Variables|Default|GetTextRender1) false false)
      (Game|Player|SetViewTargetwithBlend _player_controller (Pawn|GetControlledPawn _player_controller) 0.5 "VTBlend_Linear" 0.0 false))))

(event EventBeginPlay)

(event Collision|EventActorBeginOverlap
  (params (OtherActor :type Actor%20Object%20Reference)))

(event EventTick
  (params (DeltaSeconds :type Float%20%28single-precision%29)))

(fn ConstructionScript)

(fn NewFunction)